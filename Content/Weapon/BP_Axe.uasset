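; BP_Axe is a melee axe weapon that attaches to a character and damages what it overlaps.
; AttachToCharacter stores the wielder and snaps the axe to the "axe" socket on that character's mesh.
; DoDamage polls the Axe component's overlapping actors on demand, skips the wielder, and applies fixed damage credited to the wielder's controller.
; It returns after the first valid target, so each call hits at most one actor.
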(fn `AttachToCharacter`
  (params (NewParam :type "Character Object Reference"))
  (returns (bResult :type Boolean))
  (bind _output_get (set `self.Character` NewParam))
  (`self.K2_AttachToComponent` (`Character.Mesh` _output_get) "axe" "SnapToTarget" "SnapToTarget" "KeepRelative")
  (return true))

(fn `DoDamage`
  (returns (bResult :type Boolean))
  (bind _character (`self.Character`))
  (for _array_element (`PrimitiveComponent.GetOverlappingActors` (`self.Axe`) "/Script/Engine.Actor")
    (if (!= _array_element _character)
      (`GameplayStatics.ApplyDamage` _array_element 10.0 (`Pawn.GetController` _character) self)
      (return false))))

(fn `UserConstructionScript`)